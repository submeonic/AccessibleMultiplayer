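; BP_ClawFloor is a floor marker that follows the Xbox and Arduino ball controllers and shows claw state through its material.
; Each tick it eases toward the point nearest world origin on the line between both balls, at a fixed height, unless StopTracking is set.
; Any overlap turns it blue and flags the player as on it; ending overlap restores the grid.
; While flagged with ClawRef low, it turns red and stops moving.
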(event OnComponentBeginOverlap(ClawMesh)
  (params (OverlappedComponent :type Primitive%20Component%20Object%20Reference) (OtherActor :type Actor%20Object%20Reference) (OtherComp :type Primitive%20Component%20Object%20Reference) (OtherBodyIndex :type Integer) (bFromSweep :type Boolean) (SweepResult :type Hit%20Result%20Structure%20%28by%20ref%29))
  ;[1 1 1] Changes the material of claw on overlap of player character
  (if true
    (Variables|Default|SetIsPlayerOnFloor true)
    (Rendering|Material|SetMaterial (Variables|Default|GetClawMesh) 0 "/Game/ClawMats/MI_Solid_Blue.MI_Solid_Blue")))

(event OnComponentEndOverlap(ClawMesh)
  (params (OverlappedComponent :type Primitive%20Component%20Object%20Reference) (OtherActor :type Actor%20Object%20Reference) (OtherComp :type Primitive%20Component%20Object%20Reference) (OtherBodyIndex :type Integer))
  ;[1 1 1] Changes the material of claw on overlap of player character
  (if true
    (Variables|Default|SetIsPlayerOnFloor false)
    (Rendering|Material|SetMaterial (Variables|Default|GetClawMesh) 0 "/Game/ClawMats/MI_PrototypeGrid_TopDark.MI_PrototypeGrid_TopDark")))

(event EventBeginPlay
  (bind _returnvalue (Actor|GetActorOfClass "/Game/BP_XboxBallController.BP_XboxBallController_C"))
  (Variables|Default|SetXboxController _returnvalue)
  (bind _returnvalue_2 (Actor|GetActorOfClass "/Game/BP_BallController.BP_BallController_C"))
  (Variables|Default|SetArduinoController _returnvalue_2))

(event EventTick
  (params (DeltaSeconds :type Float%20%28single-precision%29))
  (bind _xboxcontroller (Variables|Default|GetXboxController))
  (bind _arduinocontroller (Variables|Default|GetArduinoController))
  (bind _returnvalue (Transformation|GetActorLocation _xboxcontroller))
  (bind _returnvalue_2 (Transformation|GetActorLocation _arduinocontroller))
  (bind _returnvalue_3 (Math|Vector|FindClosestPointonSegment "0, 0, 0" _returnvalue _returnvalue_2))
  (bind (_x _y) (Math|Vector|BreakVector _returnvalue_3))
  ;[1 1 1] Changes Color of Floor to Red if Z is below 500
  (if (and (< (.Z (Math|Vector|BreakVector (Transformation|GetActorLocation (Variables|Default|GetClawRef)))) 5e+02) (Variables|Default|GetIsPlayerOnFloor))
    (Rendering|Material|SetMaterial (Variables|Default|GetClawMesh) 0 "/Game/ClawMats/MI_SolidRed.MI_SolidRed")
    (else
      ;[1 1 1] Tracking Movement of ClawFloor to PlayerCharacter
      (if (not (Variables|Default|GetStopTracking))
        (Transformation|SetActorLocation (Math|Interpolation|VInterpTo (Transformation|GetActorLocation) (Math|Vector|MakeVector _x _y -9e+01) DeltaSeconds (Variables|Default|GetMovementSpeed)) false false)))))

(fn ConstructionScript)