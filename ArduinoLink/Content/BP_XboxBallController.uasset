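; BP_XboxBallController is an actor that moves a physics sphere from joystick input, named for an Xbox controller.
; BeginPlay enables input from player controller 0.
; Each Tick samples both joystick axes with X negated, then applies them, scaled by ForceMultiplier, as a horizontal force on the Sphere.
; The force is mass-dependent and is not scaled by delta time.
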(event EventTick
  (params (DeltaSeconds :type Float%20%28single-precision%29))
  (bind _forcemultiplier (Variables|Default|GetForceMultiplier))
  (Utilities|FlowControl|Sequence
    (:then_0
      (Variables|Default|SetX_Val (* -1.0 (Input|AxisValues|GetJoystick_X)))
      (Variables|Default|SetY_Val (Input|AxisValues|GetJoystick_Y)))
    (:then_1
      (Physics|AddForce (Variables|Default|GetSphere) (Math|Vector|MakeVector (* (Variables|Default|GetX_Val) _forcemultiplier) (* (Variables|Default|GetY_Val) _forcemultiplier) 0.0) "None" false))))

(event EventBeginPlay
  (Input|EnableInput (Game|GetPlayerController 0)))

(fn ConstructionScript)