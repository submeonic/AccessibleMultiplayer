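; Floor marker for the two-player claw minigame that follows the claw's XY at a fixed height and damages players standing on it.
; Overlap turns it red and flags the Xbox ball as Player 1 or the Arduino ball as Player 2.
; A Delay on Tick throttles damage to roughly once per second and refreshes the health widget.
; When either health runs out, it records the winner in GI_Marble, shows the completion widget and pauses.
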(event OnComponentBeginOverlap(ClawMesh)
  (params (OverlappedComponent :type Primitive%20Component%20Object%20Reference) (OtherActor :type Actor%20Object%20Reference) (OtherComp :type Primitive%20Component%20Object%20Reference) (OtherBodyIndex :type Integer) (bFromSweep :type Boolean) (SweepResult :type Hit%20Result%20Structure%20%28by%20ref%29))
  ;[1 1 1] Changes the material of claw on overlap of player character
  (if true
    (Variables|Default|SetIsPlayerOnFloor true)
    (Rendering|Material|SetMaterial (Variables|Default|GetClawMesh) 0 "/Game/Claw/ClawMats/MI_SolidRed.MI_SolidRed")
    (if (== OtherActor (Variables|Default|GetXboxController))
      (Variables|Default|SetPlayer1TakingDamage true))
    (if (== OtherActor (Variables|Default|GetArduinoController))
      (Variables|Default|SetPlayer2TakingDamage true))))

(event OnComponentEndOverlap(ClawMesh)
  (params (OverlappedComponent :type Primitive%20Component%20Object%20Reference) (OtherActor :type Actor%20Object%20Reference) (OtherComp :type Primitive%20Component%20Object%20Reference) (OtherBodyIndex :type Integer))
  ;[1 1 1] Changes the material of claw on overlap of player character
  (if true
    (Variables|Default|SetIsPlayerOnFloor false)
    (Rendering|Material|SetMaterial (Variables|Default|GetClawMesh) 0 "/Game/Claw/ClawMats/MI_Solid_Blue.MI_Solid_Blue")
    (if (== OtherActor (Variables|Default|GetXboxController))
      (Variables|Default|SetPlayer1TakingDamage false))
    (if (== OtherActor (Variables|Default|GetArduinoController))
      (Variables|Default|SetPlayer2TakingDamage false))))

(event Custom|SetHealthText_Event
  (Variables|/Script/UMG.TextBlock|SetText (Variables|/Game/Widgets/WB_PlayerHealthClaw.WB_PlayerHealthClaw_C|GetPlayer1HealthText (stale EventBeginPlay _returnvalue)) (Utilities|Text|ToText(Float) (Variables|Default|GetPlayer1Health) "HalfToEven"))
  (Variables|/Script/UMG.TextBlock|SetText (Variables|/Game/Widgets/WB_PlayerHealthClaw.WB_PlayerHealthClaw_C|GetPlayer2HealthText (stale EventBeginPlay _returnvalue)) (Utilities|Text|ToText(Float) (Variables|Default|GetPlayer2Health) "HalfToEven")))

(event Custom|GameWon_Event
  (bind _asgi_marble (Utilities|Casting|CastToGI_Marble (Game|GetGameInstance)))
  (Variables|/Game/GI_Marble.GI_Marble_C|SetPlayerWin _asgi_marble (Variables|Default|GetPlayerNum))
  (bind _returnvalue (UserInterface|CreateWidget "/Game/Widgets/WB_MinigameComplete.WB_MinigameComplete_C"))
  (Default|MinigameWinnerEvent _returnvalue)
  (UserInterface|Viewport|AddtoViewport _returnvalue 0)
  (Game|SetGamePaused true))

(event EventBeginPlay
  (bind _startinghealth (Variables|Default|GetStartingHealth))
  (Variables|Default|SetPlayer1Health _startinghealth)
  (Variables|Default|SetPlayer2Health _startinghealth)
  (bind _returnvalue (UserInterface|CreateWidget "/Game/Widgets/WB_PlayerHealthClaw.WB_PlayerHealthClaw_C"))
  (UserInterface|Viewport|AddtoViewport _returnvalue 0)
  (CallFunction|SetHealthTextEvent)
  (Variables|Default|SetStartLocation (Transformation|GetActorLocation))
  (bind _returnvalue_2 (Actor|GetActorOfClass "/Game/Blueprints/BP_XboxBallController.BP_XboxBallController_C"))
  (Variables|Default|SetXboxController _returnvalue_2)
  (bind _returnvalue_3 (Actor|GetActorOfClass "/Game/Blueprints/BP_BallController.BP_BallController_C"))
  (Variables|Default|SetArduinoController _returnvalue_3))

(event EventTick
  (params (DeltaSeconds :type Float%20%28single-precision%29))
  (bind _clawref (Variables|Default|GetClawRef))
  (bind _returnvalue (Transformation|GetActorLocation _clawref))
  (bind (_x _y) (Math|Vector|BreakVector _returnvalue))
  ;[1 1 1] Tracking Movement of ClawFloor to PlayerCharacter
  (Transformation|SetActorLocation (Math|Vector|MakeVector _x _y (.Z (Math|Vector|BreakVector (Variables|Default|GetStartLocation)))) false false)
  (if (<= (Variables|Default|GetPlayer1Health) 0.0)
    (Variables|Default|SetPlayerNum 1)
    (CallFunction|GameWonEvent :!label _label)
    (elif (<= (Variables|Default|GetPlayer2Health) 0.0)
      (Variables|Default|SetPlayerNum 0)
      (goto _label)
      (else
        (Utilities|FlowControl|Delay 1.0)
        (if (Variables|Default|GetPlayer1TakingDamage)
          (Math|Float|DecrementFloat (Variables|Default|GetPlayer1Health)
            (:%20%20
              (CallFunction|SetHealthTextEvent))))
        (if (Variables|Default|GetPlayer2TakingDamage)
          (Math|Float|DecrementFloat (Variables|Default|GetPlayer2Health)
            (:%20%20
              (CallFunction|SetHealthTextEvent))))))))

(fn ConstructionScript)