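; BP_Claw is a claw actor that takes over the first player's view and chases the nearer of two ball controllers, Xbox or Arduino.
; After a start delay, Tick pins the camera overhead and interpolates the claw toward that controller at fixed height, unless StopTracking is set.
; Controller lookup, the descend timeline and the capture-and-teleport logic are disconnected, leaving CheckClawPosition a no-op.
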(event EventBeginPlay
  (Game|Player|SetViewTargetwithBlend (Game|GetPlayerController 0) self 0.0 "VTBlend_Linear" 0.0 false))

(event EventTick
  (params (DeltaSeconds :type Float%20%28single-precision%29))
  (bind _returnvalue (Transformation|GetActorLocation))
  (bind _self self)
  (bind _xboxcontroller (Variables|Default|GetXboxController))
  (bind _arduinocontroller (Variables|Default|GetArduinoController))
  (bind (_x _y) (Math|Vector|BreakVector _returnvalue))
  (bind _returnvalue_2 (Transformation|GetActorLocation _xboxcontroller))
  (bind _returnvalue_3 (Transformation|GetActorLocation _self))
  (bind _returnvalue_4 (Transformation|GetActorLocation _arduinocontroller))
  (bind (_x_2 _y_2) (Math|Vector|BreakVector _returnvalue_2))
  (bind (_x_3 _y_3) (Math|Vector|BreakVector _returnvalue_4))
  (if (Variables|Default|GetCanStart)
    ;[1 1 1] Tracking Movement of Claw to PlayerCharacter
    (Transformation|SetWorldLocation (Variables|Default|GetCamera) (Math|Vector|MakeVector _x _y 4.1e+03) false false)
    (if (not (Variables|Default|GetStopTracking))
      (CallFunction|CheckClawPosition)
      (if (< (Math|Vector|Distance(Vector) _returnvalue_2 _returnvalue_3) (Math|Vector|Distance(Vector) _returnvalue_4 _returnvalue_3))
        (Transformation|SetActorLocation (Math|Interpolation|VInterpTo (Transformation|GetActorLocation) (Math|Vector|MakeVector _x_2 _y_2 1.13e+03) DeltaSeconds (Variables|Default|GetMovementSpeed)) false false)
        (else
          (Transformation|SetActorLocation (Math|Interpolation|VInterpTo (Transformation|GetActorLocation) (Math|Vector|MakeVector _x_3 _y_3 1.13e+03) DeltaSeconds (Variables|Default|GetMovementSpeed)) false false))))
    (else
      (Utilities|FlowControl|Delay 2.5)
      (Variables|Default|SetCanStart true))))

(fn ConstructionScript)

(fn CheckClawPosition)