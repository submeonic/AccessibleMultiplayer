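; BP_Marble is the physics marble in a maze minigame, respawning when it falls and reporting a player win.
; BeginPlay stores the start location, and Tick calls BallFall when height drops below RespawnHeight, moving the marble back and zeroing its linear velocity.
; CallGameWon_Event writes its PlayerNum as the winner on GI_Marble and fires that game instance's minigame completed event.
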(event Custom|CallGameWon_Event
  (bind _asgi_marble (Utilities|Casting|CastToGI_Marble (Game|GetGameInstance)))
  (Variables|/Game/GI_Marble.GI_Marble_C|SetPlayerWin _asgi_marble (Variables|Default|GetPlayerNum))
  (Default|MinigameCompletedEvent _asgi_marble))

(event EventBeginPlay
  (Variables|Default|SetStartingLocation (Transformation|GetActorLocation)))

(event EventTick
  (params (DeltaSeconds :type Float%20%28single-precision%29))
  (if (< (.z (Transformation|GetActorLocation)) (Variables|Default|GetRespawnHeight))
    (CallFunction|BallFall)))

(fn ConstructionScript)

(fn BallFall
  (Transformation|SetActorLocation (Variables|Default|GetStartingLocation) false false)
  (Physics|SetPhysicsLinearVelocity (Variables|Default|GetMarble) "0, 0, 0" false "None"))