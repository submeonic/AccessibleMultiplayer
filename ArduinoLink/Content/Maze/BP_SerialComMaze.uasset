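; BP_SerialComMaze is a maze actor that tilts its mesh from two-axis input, likely serial-fed given its name.
; On BeginPlay it finds the InputControl actor, then each Tick reads and clamps its X and Y values.
; Inverted Y drives world pitch and X drives local roll, both scaled by RotationSpeed per frame without delta time.
; Each rotation is then clamped to a few degrees either way to limit the tilt.
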(event EventBeginPlay
  (bind _returnvalue (Actor|GetActorOfClass "/Game/InputControl.InputControl_C")))

(event EventTick
  (params (DeltaSeconds :type Float%20%28single-precision%29))
  (bind _mazemesh (Variables|Default|GetMazeMesh))
  (bind _returnvalue (Transformation|GetWorldRotation _mazemesh))
  (bind _relativerotation (Variables|/Script/Engine.SceneComponent|GetRelativeRotation _mazemesh))
  (Utilities|FlowControl|Sequence
    (:then_0
      (Variables|Default|SetX_Val (Math|Float|Clamp(Float) (Variables|/Game/InputControl.InputControl_C|GetX_Val (stale EventBeginPlay _returnvalue)) -1.0))
      (Variables|Default|SetY_Val (Math|Float|Clamp(Float) (Variables|/Game/InputControl.InputControl_C|GetY_Val (stale EventBeginPlay _returnvalue)) -1.0)))
    (:then_1
      (Transformation|AddWorldRotation (Variables|Default|GetMazeMesh) (Math|Rotator|MakeRotator 0.0 (* (* (Variables|Default|GetY_Val) -1.0) (Variables|Default|GetRotationSpeed)) 0.0) false false)
      (Transformation|SetWorldRotation (Variables|Default|GetMazeMesh) (Math|Rotator|MakeRotator (.roll _returnvalue) (Math|Float|Clamp(Float) (.pitch _returnvalue) -5.0 5.0) (.yaw _returnvalue)) false false))
    (:then_2
      (Transformation|AddLocalRotation (Variables|Default|GetMazeMesh) (Math|Rotator|MakeRotator (* (Variables|Default|GetX_Val) (Variables|Default|GetRotationSpeed)) 0.0 0.0) false false)
      (Transformation|SetRelativeRotation (Variables|Default|GetMazeMesh) (Math|Rotator|MakeRotator (Math|Float|Clamp(Float) (.roll _relativerotation) -5.0 5.0) (.pitch _relativerotation) (.yaw _relativerotation)) false false))))

(fn ConstructionScript)