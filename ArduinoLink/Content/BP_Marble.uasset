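; BP_Marble is a marble actor that returns to its starting point when it falls too low.
; BeginPlay records the actor's location as StartingLocation, and Tick checks whether its Z has dropped below RespawnHeight.
; When it has, BallFall moves the actor back to that location and zeroes the Marble component's linear physics velocity.
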(event EventBeginPlay
  (Variables|Default|SetStartingLocation (Transformation|GetActorLocation)))

(event Collision|EventActorBeginOverlap
  (params (OtherActor :type Actor%20Object%20Reference)))

(event EventTick
  (params (DeltaSeconds :type Float%20%28single-precision%29))
  (if (< (.z (Transformation|GetActorLocation)) (Variables|Default|GetRespawnHeight))
    (CallFunction|BallFall)))

(fn ConstructionScript)

(fn BallFall
  (Transformation|SetActorLocation (Variables|Default|GetStartingLocation) false false)
  (Physics|SetPhysicsLinearVelocity (Variables|Default|GetMarble) "0, 0, 0" false "None"))