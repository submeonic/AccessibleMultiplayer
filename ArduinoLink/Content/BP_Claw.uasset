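; Claw hazard that owns the player camera, follows the two ball controllers (Xbox and Arduino) and catches a player on the claw floor.
; Tick holds the camera overhead and interpolates the claw toward the point on the segment between both balls nearest the world origin.
; A timeline started at BeginPlay drives its height.
; When the claw is low and a player is on the floor, it teleports the ball nearest the floor away and stops tracking.
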(event EventBeginPlay
  (bind _returnvalue (Transformation|GetActorLocation))
  (bind (_x _y) (Math|Vector|BreakVector _returnvalue))
  (Game|Player|SetViewTargetwithBlend (Game|GetPlayerController 0) self 0.0 "VTBlend_Linear" 0.0 false)
  (bind _returnvalue_2 (Actor|GetActorOfClass "/Game/BP_XboxBallController.BP_XboxBallController_C"))
  (Variables|Default|SetXboxController _returnvalue_2)
  (bind _returnvalue_3 (Actor|GetActorOfClass "/Game/BP_BallController.BP_BallController_C"))
  (Variables|Default|SetArduinoController _returnvalue_3)
  ;[1 1 1] Claw moving up and down
  (Utilities|Time|SetTimerbyFunctionName 0 "" 1e+01 true)
  (bind _clawzposition (Timeline|DescendTimeline Play)
    (:Update
      (Transformation|SetActorLocation (Math|Vector|MakeVector _x _y _clawzposition) false false))
    (:Finished
      (CallFunction|DescendTimelineFinishedFunc))))

(event EventTick
  (params (DeltaSeconds :type Float%20%28single-precision%29))
  (bind _returnvalue (Transformation|GetActorLocation))
  (bind _xboxcontroller (Variables|Default|GetXboxController))
  (bind _arduinocontroller (Variables|Default|GetArduinoController))
  (bind (_x _y) (Math|Vector|BreakVector _returnvalue))
  (bind _returnvalue_2 (Transformation|GetActorLocation _xboxcontroller))
  (bind _returnvalue_3 (Transformation|GetActorLocation _arduinocontroller))
  (bind _returnvalue_4 (Math|Vector|FindClosestPointonSegment "0, 0, 0" _returnvalue_2 _returnvalue_3))
  (bind (_x_2 _y_2) (Math|Vector|BreakVector _returnvalue_4))
  ;[1 1 1] Tracking Movement of Claw to PlayerCharacter
  (Transformation|SetWorldLocation (Variables|Default|GetCamera) (Math|Vector|MakeVector _x _y 2e+03) false false)
  (if (not (Variables|Default|GetStopTracking))
    (CallFunction|CheckClawPosition)
    (Transformation|SetActorLocation (Math|Interpolation|VInterpTo (Transformation|GetActorLocation) (Math|Vector|MakeVector _x_2 _y_2 1.13e+03) DeltaSeconds (Variables|Default|GetMovementSpeed)) false false)))

(fn ConstructionScript)

(fn CheckClawPosition
  (if (and (Variables|/Game/BP_ClawFloor.BP_ClawFloor_C|GetIsPlayerOnFloor (Variables|Default|GetClawFloorRef)) (< (Math|Float|Absolute(Float) (- (.Z (Math|Vector|BreakVector (Transformation|GetActorLocation))) 1.5e+02)) 2e+01))
    (Transformation|SetActorLocation (.ReturnValue (Actor|FindNearestActor (Transformation|GetActorLocation (Variables|Default|GetClawFloorRef)) (Utilities|Array|MakeArray (Variables|Default|GetArduinoController) (Variables|Default|GetXboxController)))) (Math|Vector|MakeVector 1.71e+03 7.1e+02 3.8e+02) false true)
    ;[1 1 1] IF true, claw will stop tracking this player
    (Variables|/Game/BP_ClawFloor.BP_ClawFloor_C|SetStopTracking (Variables|Default|GetClawFloorRef) true)
    (Variables|Default|SetStopTracking true)))