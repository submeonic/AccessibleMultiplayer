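; BP_WinningBall is the marble shown on the game-won screen to represent the winning player.
; On BeginPlay it reads PlayerWin from the GI_Marble game instance.
; It then shows either the Player1 or Player2 component and hides the other.
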(event EventBeginPlay
  (CallFunction|SetWinningMarble))

(fn ConstructionScript)

(fn SetWinningMarble
  (bind _asgi_marble (Utilities|Casting|CastToGI_Marble (Game|GetGameInstance)))
  (switch int (Variables|/Game/GI_Marble.GI_Marble_C|GetPlayerWin _asgi_marble)
    (:0
      (Rendering|SetVisibility (Variables|Default|GetPlayer2) false false)
      (Rendering|SetVisibility (Variables|Default|GetPlayer1) true false))
    (:1
      (Rendering|SetVisibility (Variables|Default|GetPlayer1) false false)
      (Rendering|SetVisibility (Variables|Default|GetPlayer2) true false))))