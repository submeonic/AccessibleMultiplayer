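; BP_BallController drives a physics ball from the axis values of an InputControl actor, which it finds on BeginPlay.
; Each Tick it copies that actor's axes and button states, negating X and clamping both axes to the -1 to 1 range.
; It then pushes the Sphere horizontally with a force scaled by ForceMultiplier; the button states are stored but not used in this graph.
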(event EventBeginPlay
  (bind _returnvalue (Actor|GetActorOfClass "/Game/InputControl.InputControl_C")))

(event Collision|EventActorBeginOverlap
  (params (OtherActor :type Actor%20Object%20Reference)))

(event EventTick
  (params (DeltaSeconds :type Float%20%28single-precision%29))
  (bind _forcemultiplier (Variables|Default|GetForceMultiplier))
  (Utilities|FlowControl|Sequence
    (:then_0
      (Variables|Default|SetX_Val (Math|Float|Clamp(Float) (* (Variables|/Game/InputControl.InputControl_C|GetX_Val (stale EventBeginPlay _returnvalue)) -1.0) -1.0))
      (Variables|Default|SetY_Val (Math|Float|Clamp(Float) (Variables|/Game/InputControl.InputControl_C|GetY_Val (stale EventBeginPlay _returnvalue)) -1.0))
      (Variables|Default|SetRightButtonState (Variables|/Game/InputControl.InputControl_C|GetRightButtonState (stale EventBeginPlay _returnvalue)))
      (Variables|Default|SetLeftButtonState (Variables|/Game/InputControl.InputControl_C|GetLeftButtonState (stale EventBeginPlay _returnvalue))))
    (:then_1
      (Physics|AddForce (Variables|Default|GetSphere) (Math|Vector|MakeVector (* (Variables|Default|GetX_Val) _forcemultiplier) (* (Variables|Default|GetY_Val) _forcemultiplier) 0.0) "None" false))))

(fn ConstructionScript)