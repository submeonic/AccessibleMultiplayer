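; Ready-up hole trigger for a two-player marble game that starts the match once both players are ready.
; IsPlayer1Hole assigns the hole: BP_XboxBallController belongs in Player 1's, BP_BallController in the other.
; The right ball entering runs a readiness check, which reads both ready flags from GI_Marble and calls its StartGameEvent.
; A ball in the wrong hole is moved back to its start location cached on BeginPlay.
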(event Custom|CheckIfReady_Event
  (bind _asgi_marble (Utilities|Casting|CastToGI_Marble (Game|GetGameInstance)))
  (if (and (Variables|/Game/GI_Marble.GI_Marble_C|GetPlayer1Ready _asgi_marble) (Variables|/Game/GI_Marble.GI_Marble_C|GetPlayer2Ready _asgi_marble))
    (Default|StartGameEvent _asgi_marble)))

(event Collision|EventActorBeginOverlap
  (params (OtherActor :type Actor%20Object%20Reference))
  (Utilities|Casting|CastToBP_BallController OtherActor
    (:then
      (if (!= (Variables|Default|GetIsPlayer1Hole) true)
        (CallFunction|CheckifReadyEvent)
        (else
          (Transformation|SetActorLocation (Variables|Default|GetPlayer2) (Variables|Default|GetPlayer2StartLocation) false false))))
    (:CastFailed
      (Utilities|Casting|CastToBP_XboxBallController OtherActor)
      (if (Variables|Default|GetIsPlayer1Hole)
        (CallFunction|CheckifReadyEvent)
        (else
          (Transformation|SetActorLocation (Variables|Default|GetPlayer1) (Variables|Default|GetPlayer1StartLocation) false false))))))

(event EventBeginPlay
  (Variables|Default|SetPlayer1StartLocation (Transformation|GetActorLocation (Variables|Default|GetPlayer1)))
  (Variables|Default|SetPlayer2StartLocation (Transformation|GetActorLocation (Variables|Default|GetPlayer2))))

(fn ConstructionScript)