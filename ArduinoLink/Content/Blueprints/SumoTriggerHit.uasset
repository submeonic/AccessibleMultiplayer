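; Trigger actor, apparently for a sumo marble minigame, that ends the match when a player's ball overlaps it.
; The overlap casts to BP_BallController or BP_XboxBallController to choose a player number, then calls the game-won event.
; That event stores the number as PlayerWin in GI_Marble, shows the WB_MinigameComplete winner widget and pauses the game.
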(event Custom|GameWon_Event
  (bind _asgi_marble (Utilities|Casting|CastToGI_Marble (Game|GetGameInstance)))
  (Variables|/Game/GI_Marble.GI_Marble_C|SetPlayerWin _asgi_marble (Variables|Default|GetPlayerNum))
  (bind _returnvalue (UserInterface|CreateWidget "/Game/Widgets/WB_MinigameComplete.WB_MinigameComplete_C"))
  (Default|MinigameWinnerEvent _returnvalue)
  (UserInterface|Viewport|AddtoViewport _returnvalue 0)
  (Game|SetGamePaused true))

(event EventBeginPlay)

(event Collision|EventActorBeginOverlap
  (params (OtherActor :type Actor%20Object%20Reference))
  (Utilities|Casting|CastToBP_BallController OtherActor
    (:then
      (Variables|Default|SetPlayerNum 0)
      (CallFunction|GameWonEvent))
    (:CastFailed
      (Utilities|Casting|CastToBP_XboxBallController OtherActor)
      (Variables|Default|SetPlayerNum 1)
      (CallFunction|GameWonEvent))))

(event EventTick
  (params (DeltaSeconds :type Float%20%28single-precision%29)))

(fn ConstructionScript)