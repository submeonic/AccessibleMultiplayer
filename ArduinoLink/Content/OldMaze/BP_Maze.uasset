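; BP_Maze is a maze board that the player tilts with the Vertical_Tilt and Horizontal_Tilt input axes.
; Each axis adds rotation scaled by RotationSpeed to MazeBoardMesh, then clamps that angle to a small symmetric range.
; Vertical input drives pitch in world space, while horizontal input drives roll through local and relative rotation.
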(event Input|AxisEvents|InputAxisHorizontal_Tilt
  (params (AxisValue :type Float%20%28single-precision%29))
  (bind _maze_board_mesh (Variables|Default|GetMaze_Board_Mesh))
  (bind _relativerotation (Variables|/Script/Engine.SceneComponent|GetRelativeRotation _maze_board_mesh))
  (Transformation|AddLocalRotation (Variables|Default|GetMaze_Board_Mesh) (Math|Rotator|MakeRotator (* AxisValue (Variables|Default|GetRotationSpeed)) 0.0 0.0) false false)
  (Transformation|SetRelativeRotation (Variables|Default|GetMaze_Board_Mesh) (Math|Rotator|MakeRotator (Math|Float|Clamp(Float) (.roll _relativerotation) -5.0 5.0) (.pitch _relativerotation) (.yaw _relativerotation)) false false))

(event Input|AxisEvents|InputAxisVertical_Tilt
  (params (AxisValue :type Float%20%28single-precision%29))
  (bind _maze_board_mesh (Variables|Default|GetMaze_Board_Mesh))
  (bind _returnvalue (Transformation|GetWorldRotation _maze_board_mesh))
  (Transformation|AddWorldRotation (Variables|Default|GetMaze_Board_Mesh) (Math|Rotator|MakeRotator 0.0 (* AxisValue (Variables|Default|GetRotationSpeed)) 0.0) false false)
  (Transformation|SetWorldRotation (Variables|Default|GetMaze_Board_Mesh) (Math|Rotator|MakeRotator (.roll _returnvalue) (Math|Float|Clamp(Float) (.pitch _returnvalue) -5.0 5.0) (.yaw _returnvalue)) false false))

(fn ConstructionScript)